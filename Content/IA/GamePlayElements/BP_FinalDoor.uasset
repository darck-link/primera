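; BP_FinalDoor is a door that opens once all collectable items have been collected.
; On BeginPlay it counts the actors of a class into RemainingCollectableItem, opening immediately if there are none.
; Each ItemCollected event decrements that counter and calls OpenDoor at zero, which simply destroys the door actor.
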(event Custom|OpenDoor
  (Actor|DestroyActor))

(event Custom|ItemCollected
  (bind _result (Math|Integer|DecrementInt (Variables|Default|Get%20RemainingCollectableItem))
    (:%20%20
      (if (== _result 0)
        (CallFunction|OpenDoor)))))

(event EventBeginPlay
  (bind _outactors (Actor|GetAllActorsOfClass 0))
  (bind _output_get (Variables|Default|Set%20RemainingCollectableItem (Utilities|Array|Length _outactors)))
  (if (== _output_get 0)
    (CallFunction|OpenDoor)))

(event Collision|EventActorBeginOverlap
  (params (OtherActor :type Actor%20Object%20Reference)))

(event EventTick
  (params (DeltaSeconds :type Float%20%28single-precision%29)))

(fn ConstructionScript)